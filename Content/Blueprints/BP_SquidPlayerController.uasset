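; Squid Game-style player controller that presents end-of-round screens for three outcomes: both players win, both die, or only one survives.
; Each outcome is a custom event guarded by its own DoOnce.
; The win event waits briefly, shows the all-won widget and end screen with a sound, then opens the GreenLightRedLight level after another delay.
; Both-die and one-survivor events only add the shared end screen.
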(event `self.AnnounceBothPlayersAsWinner`
  ;[0.02022 1 0 0.5] Both Player Win
  (`/Engine/EditorBlueprintResources/StandardMacros.DoOnce` false
    (:`Completed`
      (`KismetSystemLibrary.Delay` 3.0)
      (bind _returnvalue (`|CreateWidget` "/Game/UI/WPB_AllPlayerWon.WPB_AllPlayerWon_C"))
      (`UserWidget.AddToViewport` _returnvalue 1)
      (`GameplayStatics.PlaySound2D` "/Game/Audios/EndGame.EndGame" 1.0 1.0 0.0 null null)
      (bind _returnvalue_2 (`|CreateWidget` "/Game/UI/WBP_EndScreen.WBP_EndScreen_C"))
      (`UserWidget.AddToViewport` _returnvalue_2 0)
      (`KismetSystemLibrary.Delay` 5.0)
      (`GameplayStatics.OpenLevelBySoftObjectPtr` "/Game/Maps/GreenLightRedLight.GreenLightRedLight"))))

(event `self.BothPlayersDie`
  ;[1 0 0 0.5] Both Player Lose
  (`/Engine/EditorBlueprintResources/StandardMacros.DoOnce` false
    (:`Completed`
      (bind _returnvalue (`|CreateWidget` "/Game/UI/WBP_EndScreen.WBP_EndScreen_C"))
      (`UserWidget.AddToViewport` _returnvalue 0))))

(event `self.OnlyOnePlayersLives`
  ;[1 1 1 0.5] One Player Lives
  (`/Engine/EditorBlueprintResources/StandardMacros.DoOnce` false
    (:`Completed`
      (bind _returnvalue (`|CreateWidget` "/Game/UI/WBP_EndScreen.WBP_EndScreen_C"))
      (`UserWidget.AddToViewport` _returnvalue 0))))

(fn `UserConstructionScript`)