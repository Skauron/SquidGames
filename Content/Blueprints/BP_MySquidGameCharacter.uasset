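; Squid Game character Blueprint that shows the player's number on a widget and announces that player when they win.
; Every Tick it rewrites the three-digit number on NumWidget and rotates the widget to face the BP_Camera actor found in the level.
; AnnouncePlayerasWinner runs once, showing WBP_PlayerReachGoal with the player number for a few seconds before removing it.
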(event `self.ReceiveTick`
  (params (DeltaSeconds :type "Float (single-precision)"))
  ;[0 0.8318 1 0.5] Number Player
  (`self.SetNumber`)
  (`self.SetRotationToCamera`))

(event `self.AnnouncePlayerAsWinner`
  ;[0.1077 1 0 0.5] Event when player wins
  (`/Engine/EditorBlueprintResources/StandardMacros.DoOnce` false
    (:`Completed`
      (bind _returnvalue (`|CreateWidget` "/Game/UI/WBP_PlayerReachGoal.WBP_PlayerReachGoal_C"))
      (`TextBlock.SetText` (`/Game/UI/WBP_PlayerReachGoal.NumPlayer` _returnvalue) (`KismetTextLibrary.Conv_IntToText` (`self.GetPlayerNumber` self) false true 3))
      (`UserWidget.AddToViewport` _returnvalue 0)
      (`KismetSystemLibrary.Delay` 3.0)
      (`Widget.RemoveFromParent` _returnvalue))))

(fn `SetNumber`
  (bind _aswbp_num_player (cast `/Game/UI/WBP_NumPlayer` (`WidgetComponent.GetWidget` (`self.NumWidget`))))
  (`TextBlock.SetText` (`/Game/UI/WBP_NumPlayer.NumPlayer` _aswbp_num_player) (`KismetTextLibrary.Conv_IntToText` (`self.GetPlayerNumber` self) false true 3)))

(fn `SetRotationToCamera`
  (bind _numwidget (`self.NumWidget`))
  (bind _returnvalue (`GameplayStatics.GetActorOfClass` "/Game/Blueprints/Actors/BP_Camera.BP_Camera_C"))
  (`SceneComponent.K2_SetWorldRotation` _numwidget (`KismetMathLibrary.FindLookAtRotation` (`SceneComponent.K2_GetComponentLocation` _numwidget) (`SceneComponent.K2_GetComponentLocation` (`Actor.RootComponent` _returnvalue))) false false))

(fn `UserConstructionScript`)